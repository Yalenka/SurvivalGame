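; Survival character Blueprint with modular body meshes following the main skeleton, montage hit reactions with blood, and a slot-based weapon system.
; AttemptToAddWeapon attaches pickups to back sockets via a slot map initialized at BeginPlay.
; AttemptEquipWeapon swaps weapons between back and hands on montage notifies, recursing after unequip, with animations multicast to remote roles.
; Equip, trace-interact and default-item calls are unwired here; X prints nearby pickups for debugging.
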(event `self.ReceivePointDamage`
  (params (Damage :type "Float (single-precision)") (DamageType :type "DamageType Object Reference") (HitLocation :type "Vector Structure") (HitNormal :type "Vector Structure") (HitComponent :type "PrimitiveComponent Object Reference") (BoneName :type Name) (ShotFromDirection :type "Vector Structure") (InstigatedBy :type "Controller Object Reference") (DamageCauser :type "Actor Object Reference") (HitInfo :type "HitResult Structure (by ref)"))
  (`self.Play Hit FX` Damage DamageType HitInfo true))

(event `Play Hit FX`
  (params (Damage :type "Float (double-precision)") (`Damage Type` :type "DamageType Object Reference") (Hit :type "HitResult Structure") (`Point Damage?` :type Boolean))
  (bind (_bblockinghit _binitialoverlap _time _distance _location _impactpoint _normal _impactnormal) (`GameplayStatics.BreakHitResult` Hit))
  (bind _hitreactanimations (`self.HitReactAnimations`))
  (`self.PlayAnimMontage` (`|GetArrayItem` _hitreactanimations (`KismetMathLibrary.RandomIntegerInRange` 0 (- (`KismetArrayLibrary.Array_Length` _hitreactanimations) 1))))
  (if `Point Damage?`
    (`GameplayStatics.SpawnEmitterAtLocation` "/Game/Particles/P_Blood.P_Blood" _location (`KismetMathLibrary.Conv_VectorToRotator` _impactnormal))))

(event `Key|X`
  (params (Key :type "Key Structure"))
  (:`Pressed`
    (bind _outactors (`KismetSystemLibrary.SphereOverlapActors` (`self.K2_GetActorLocation`) 500.0 (`|MakeArray` "ObjectTypeQuery2" :!type "EObjectTypeQuery Enum") "/Game/Blueprints/BP_PickupBase.BP_PickupBase_C"))
    (for _array_element _outactors
      (`KismetSystemLibrary.PrintString` (`KismetSystemLibrary.GetDisplayName` _array_element)))))

(event `self.PlayerInventory.OnItemAdded`
  (params (Item :type "Item Object Reference")))

(event `MC  Weapon Animations`
  (params (MontageToPlay :type "AnimMontage Object Reference"))
  ;[1 1 1] Multicast Animation (only clients should do this for equipping and unequipping weapons)
  (`/Engine/EditorBlueprintResources/ActorMacros.Switch Has Authority`
    (:`Remote`
      (`/Engine/EditorBlueprintResources/StandardMacros.IsValid` MontageToPlay
        (:`Is Valid`
          (`|PlayMontage` (`self.Mesh`) MontageToPlay))))))

(event `self.ReceiveBeginPlay`
  ;[1 1 1] Beginplay
  (`self.InitializeWeaponSlot`))

(event `Server Interact`
  (bind _returnvalue (`GameplayStatics.GetPlayerCameraManager` 0))
  (bind _returnvalue_2 (`PlayerCameraManager.GetCameraLocation` _returnvalue))
  ;[1 1 1] Server interaction (you should not need this, you should use the cpp interaction instead, and just call "attempt to add weapon" function
  (bind (_outhit _returnvalue_3) (`KismetSystemLibrary.LineTraceSingle` :`Start` _returnvalue_2 :`End` (+ _returnvalue_2 (* (`KismetMathLibrary.GetForwardVector` (`PlayerCameraManager.GetCameraRotation` _returnvalue)) 1000.0)) :`TraceChannel` "TraceTypeQuery1" :`DrawDebugType` "ForDuration"))
  (if _returnvalue_3
    (bind _asbp_pickup_base (cast `/Game/Blueprints/BP_PickupBase` (`.HitActor` (`GameplayStatics.BreakHitResult` _outhit))))
    (`self.AttemptToAddWeapon` _asbp_pickup_base) ; Add weapon
  ))

(event `InputAction|Interact`
  (params (Key :type "Key Structure"))
  ;[1 1 1] Interaction
)

(event `InputAction|KeyboardOneKey`
  (params (Key :type "Key Structure"))
  ;[1 1 1] Input Actions
)

(event `Attempt Equip Weapon`
  (params (Slot :type "WeaponSlot Enum" :default "Primary"))
  ;[1 1 1] Attempt to equip
  (set `self.CanChangeWeapon` false) ; TurnOffAbilityToChangeWeapons
  ;;[1 1 1] A simple check to make sure you don't unequip and requip the same weapon twice
  (if (`|EnumInequality` Slot (`self.LastEquippedSlot`))
    ;;[1 1 1] Check if a weapon is already held
    (`/Engine/EditorBlueprintResources/StandardMacros.IsValid` (`self.CurrentlyHeldWeapon`)
      (:`Is Valid`
        ;;[1 1 1] Unequip Logic
        ;;;[1 1 1] Multicast animation, and server play animation
        (`self.MC  Weapon Animations` "/Game/Blueprints/Character/Montage/AS_Stand_UnEquip_Montage.AS_Stand_UnEquip_Montage")
        (bind _notifyname (`|PlayMontage` (`self.Mesh`) "/Game/Blueprints/Character/Montage/AS_Stand_UnEquip_Montage.AS_Stand_UnEquip_Montage")
          (:`OnNotifyBegin`
            (switch `name` _notifyname ; Start unequiping
              (:`Unequip`
                ;;;[1 1 1] Find the available slot to put the gun in
                (bind _result (`BlueprintSetLibrary.Set_ToArray` (`/Game/Blueprints/BP_PickupBase.PlaceableSlots` (`self.CurrentlyHeldWeapon`))))
                (bind (_slot_found _slot _socket) (`self.Find Available Slot` _result))
                (if _slot_found
                  ;;;[1 1 1] Add weapon to slot
                  (`BlueprintMapLibrary.Map_Add` (`self.WeaponSlots`) _slot (`self.CurrentlyHeldWeapon`))
                  ;;;[1 1 1] Attach weapon to back
                  (`self.K2_AttachToComponent` (`self.CurrentlyHeldWeapon`) (`self.Mesh`) _socket "SnapToTarget" "SnapToTarget" "KeepRelative" true)
                  (set `self.CurrentlyHeldWeapon` null) ; clear currently held weapon variable
                  (`KismetSystemLibrary.Delay` 0.1) ; wait some time before equipping
                  (`self.Attempt Equip Weapon` Slot)
                  (else
                    (`KismetSystemLibrary.PrintString` "Error:: No Slot Available" true true (struct :`R` 1.0 :`G` 0.005895 :`A` 1.0) 5.0))))))))
      (:`Is Not Valid`
        ;;[1 1 1] Equip Logic
        ;;;[1 1 1] Set the last equipped slot
        (set `self.LastEquippedSlot` Slot)
        ;;;[1 1 1] First check there is a valid gun to equip in our weapon slot
        (`/Engine/EditorBlueprintResources/StandardMacros.IsValid` (`BlueprintMapLibrary.Map_Find` (`self.WeaponSlots`) Slot)
          (:`Is Valid`
            ;;;[1 1 1] Multicast animation, and server play animation
            (`self.MC  Weapon Animations` "/Game/Blueprints/Character/Montage/AS_Stand_Equip_Montage.AS_Stand_Equip_Montage")
            (bind _notifyname_2 (`|PlayMontage` (`self.Mesh`) "/Game/Blueprints/Character/Montage/AS_Stand_Equip_Montage.AS_Stand_Equip_Montage")
              (:`OnNotifyBegin`
                (switch `name` _notifyname_2 ; start equipping
                  (:`Equip`
                    ;;;[1 1 1] Set the currently held weapon
                    (set `self.CurrentlyHeldWeapon` (`BlueprintMapLibrary.Map_Find` (`self.WeaponSlots`) Slot))
                    ;;;[1 1 1] Clear the weapon slot
                    (`BlueprintMapLibrary.Map_Add` (`self.WeaponSlots`) Slot)
                    ;;;[1 1 1] Attach currently help weapon to hands
                    (`self.K2_AttachToComponent` (`self.CurrentlyHeldWeapon`) (`self.Mesh`) (`self.Get Socket Name From Slot` Slot true) "SnapToTarget" "SnapToTarget" "KeepRelative" true)
                    (set `self.CanChangeWeapon` true) ; TurnOnAbilityToChangeWeapons
                  )))))
          (:`Is Not Valid`
            (`KismetSystemLibrary.PrintString` "No Weapon In Slot" true true (struct :`R` 1.0 :`G` 0.884102 :`A` 1.0) 3.0)
            (set `self.CanChangeWeapon` true) ; TurnOnAbilityToChangeWeapons
          ))))
    (else
      ;;[1 1 1] If you try to equip the same weapon twice, then just equip nothing
      (`self.Attempt Equip Weapon` "None"))))

(event `InputAction|KeyboardTwoKey`
  (params (Key :type "Key Structure"))
  ;[1 1 1] Input Actions
)

(fn `AttemptToAddWeapon`
  (params (Weapon :type "/Game/Blueprints/BP_PickupBase Object Reference"))
  (`/Engine/EditorBlueprintResources/StandardMacros.IsValid` Weapon
    (:`Is Valid`
      ;[1 1 1] Conver placeable slots to array
      (bind _result (`BlueprintSetLibrary.Set_ToArray` (`/Game/Blueprints/BP_PickupBase.PlaceableSlots` (`local.Weapon`))))
      (bind (_slot_found _slot _socket) (`self.Find Available Slot` _result))
      (if _slot_found
        ;[1 1 1] Add weapon to slots and attach to back
        (`BlueprintMapLibrary.Map_Add` (`self.WeaponSlots`) _slot (`local.Weapon`))
        (`self.K2_AttachToComponent` (`local.Weapon`) (`self.Mesh`) _socket "SnapToTarget" "SnapToTarget" "KeepRelative" true)
        (else
          (`KismetSystemLibrary.PrintString` "No available slot found" true true (struct :`R` 1.0 :`G` 0.902084 :`A` 1.0)))))
    (:`Is Not Valid`
      (`KismetSystemLibrary.PrintString` "Error:: Tried to equip nothing" true true (struct :`R` 1.0 :`G` 0.01394 :`A` 1.0) 4.0))))

(fn `Find Available Slot`
  (params (PlaceableSlots :type "Array of WeaponSlot Enum") (Equip :type Boolean))
  (returns (`Slot Found` :type Boolean) (Slot :type "WeaponSlot Enum") (Socket :type Name))
  ;[1 1 1] Loop through all of the weapon slots
  (bind _keys (`BlueprintMapLibrary.Map_Keys` (`self.WeaponSlots`)))
  (for _array_element _keys
    ;[1 1 1] Check if the value is valid
    (`/Engine/EditorBlueprintResources/StandardMacros.IsValid` (`BlueprintMapLibrary.Map_Find` (`self.WeaponSlots`) _array_element)
      (:`Is Not Valid`
        ;[1 1 1] If it's not valid, check if the weapon slot matches the placeable slot
        (if (`KismetArrayLibrary.Array_Contains` (`local.PlaceableSlots`) _array_element)
          (return true _array_element (`self.Get Socket Name From Slot` _array_element Equip))))))
  (return false "Primary" "None"))

(fn `Get Socket Name From Slot`
  (params (Slot :type "WeaponSlot Enum" :default "Primary") (Equip :type Boolean))
  (returns (ReturnValue :type Name))
  (if Equip
    (return "Socket_Gun_Stand")
    (else
      (return (select `WeaponSlot` Slot :`Primary` "Socket_BackLeft_Normal" :`Secondary` "Socket_BackRight_Normal" :!type "Name")))))

(fn `InitializeWeaponSlot`
  (bind _enumvalue (foreach `WeaponSlot` false)
    (:`LoopBody`
      (`BlueprintMapLibrary.Map_Add` (`self.WeaponSlots`) _enumvalue))))

(fn `UserConstructionScript`
  (`SkinnedMeshComponent.SetLeaderPoseComponent` (`self.FullBody`) (`self.Mesh`) false)
  (`SkinnedMeshComponent.SetLeaderPoseComponent` (`self.FeetMesh`) (`self.Mesh`) false)
  (`SkinnedMeshComponent.SetLeaderPoseComponent` (`self.LegsMesh`) (`self.Mesh`) false)
  (`SkinnedMeshComponent.SetLeaderPoseComponent` (`self.ChestMesh`) (`self.Mesh`) false)
  (`SkinnedMeshComponent.SetLeaderPoseComponent` (`self.HandsMesh`) (`self.Mesh`) false))