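; Survival character Blueprint that adds hit feedback and a starting inventory.
; Point damage feeds PlayHitFX, which plays a random hit-react montage and spawns blood at the impact, oriented to the surface normal.
; After a short delay on BeginPlay, the authority adds DefaultItems to PlayerInventory.
; The X key runs a debug sphere overlap that prints nearby pickup names; the item-added handler is empty.
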(event `self.ReceivePointDamage`
  (params (Damage :type "Float (single-precision)") (DamageType :type "DamageType Object Reference") (HitLocation :type "Vector Structure") (HitNormal :type "Vector Structure") (HitComponent :type "PrimitiveComponent Object Reference") (BoneName :type Name) (ShotFromDirection :type "Vector Structure") (InstigatedBy :type "Controller Object Reference") (DamageCauser :type "Actor Object Reference") (HitInfo :type "HitResult Structure (by ref)"))
  (`self.Play Hit FX` Damage DamageType HitInfo true))

(event `Play Hit FX`
  (params (Damage :type "Float (double-precision)") (`Damage Type` :type "DamageType Object Reference") (Hit :type "HitResult Structure") (`Point Damage?` :type Boolean))
  (bind (_bblockinghit _binitialoverlap _time _distance _location _impactpoint _normal _impactnormal) (`GameplayStatics.BreakHitResult` Hit))
  (bind _hitreactanimations (`self.HitReactAnimations`))
  (`self.PlayAnimMontage` (`|GetArrayItem` _hitreactanimations (`KismetMathLibrary.RandomIntegerInRange` 0 (- (`KismetArrayLibrary.Array_Length` _hitreactanimations) 1))))
  (if `Point Damage?`
    (`GameplayStatics.SpawnEmitterAtLocation` "/Game/Particles/P_Blood.P_Blood" _location (`KismetMathLibrary.Conv_VectorToRotator` _impactnormal))))

(event `self.PlayerInventory.OnItemAdded`
  (params (Item :type "Item Object Reference")))

(event `self.ReceiveBeginPlay`
  (`KismetSystemLibrary.Delay` 1.0)
  (`/Engine/EditorBlueprintResources/ActorMacros.Switch Has Authority`
    (:`Authority`
      (for _array_element (`self.DefaultItems`)
        (`InventoryComponent.TryAddItemFromClass` (`self.PlayerInventory`) _array_element 999)))))

(event `Key|X`
  (params (Key :type "Key Structure"))
  (:`Pressed`
    (bind _outactors (`KismetSystemLibrary.SphereOverlapActors` (`self.K2_GetActorLocation`) 500.0 (`|MakeArray` "ObjectTypeQuery2" :!type "EObjectTypeQuery Enum") "/Game/Blueprints/BP_PickupBase.BP_PickupBase_C"))
    (for _array_element _outactors
      (`KismetSystemLibrary.PrintString` (`KismetSystemLibrary.GetDisplayName` _array_element)))))

(fn `UserConstructionScript`)