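; BP_SurvivalGameInstance is the survival game's GameInstance, handling online session joining and leaving.
; TryJoinGame runs an Advanced Sessions search filtered on a "Spacewar" GAMENAME and joins the first result without an empty-list check.
; A successful join switches to game-only input and hides the cursor, while search or join failures call OnFailedToFindMatch.
; Both quit events destroy the session, then exit or open MainMenu even if destruction fails.
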(event `Try Join Game`
  (bind _results (`FindSessionsCallbackProxyAdvanced.FindSessionsAdvanced` (`GameplayStatics.GetPlayerController` 0) 1000 false "AllServers" (`|MakeArray` (`AdvancedSessionsLibrary.MakeLiteralSessionSearchProperty` (`AdvancedSessionsLibrary.MakeLiteralSessionPropertyString` "GAMENAME" "Spacewar") "Equals")))
    (:`OnSuccess`
      (`self.Join Session` (`|GetArrayItem` _results)))
    (:`OnFailure`
      (`self.OnFailedToFindMatch` "Find sessions failed"))))

(event `Quit to Desktop`
  (`DestroySessionCallbackProxy.DestroySession` (`GameplayStatics.GetPlayerController` 0)
    (:`OnSuccess`
      _)
    (:`OnFailure`
      _))
  (`KismetSystemLibrary.QuitGame` null "Quit"))

(event `Quit to Main Menu`
  (`DestroySessionCallbackProxy.DestroySession` (`GameplayStatics.GetPlayerController` 0)
    (:`OnSuccess`
      _)
    (:`OnFailure`
      _))
  (`GameplayStatics.OpenLevel` "MainMenu"))

(event `Join Session`
  (params (Session :type "BlueprintSessionResult Structure"))
  (bind _returnvalue (`GameplayStatics.GetPlayerController` 0))
  (`JoinSessionCallbackProxy.JoinSession` (`GameplayStatics.GetPlayerController` 0) Session
    (:`OnSuccess`
      (`WidgetBlueprintLibrary.SetInputMode_GameOnly` _returnvalue)
      (set `PlayerController.bShowMouseCursor` false _returnvalue))
    (:`OnFailure`
      (`self.OnFailedToFindMatch` "failed to join session"))))