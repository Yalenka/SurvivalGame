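; BP_SurvivalGameGameModeBase is the survival game mode that assigns each player a separate spawn point.
; Its FindPlayerStart override lazily fills the Starts array with every BP_SurvivalPlayerStart actor through InitStarts when the array is empty.
; It then returns the first start not yet used and marks it used so later players receive different ones.
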(event `Init Starts`
  (bind _outactors (`GameplayStatics.GetAllActorsOfClass` "/Game/Blueprints/BP_SurvivalPlayerStart.BP_SurvivalPlayerStart_C"))
  (set `self.Starts` _outactors))

(event `self.ReceiveBeginPlay`)

(fn `FindPlayerStart`
  (params (Player :type "Controller Object Reference") (IncomingName :type String))
  (returns (ReturnValue :type "Actor Object Reference"))
  (locals (PlayerStart :type "/Game/Blueprints/BP_SurvivalPlayerStart Object Reference"))
  (if (<= (`KismetArrayLibrary.Array_Length` (`self.Starts`)) 0)
    (`self.Init Starts`))
  (for _array_element (`self.Starts`)
    (if (not (`/Game/Blueprints/BP_SurvivalPlayerStart.Used` _array_element))
      (`/Game/Blueprints/BP_SurvivalPlayerStart.Mark Used` _array_element)
      (return _array_element))))

(fn `UserConstructionScript`)