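; BP_SurvivalPlayerController is the survival game's player controller that toggles the inventory screen on the ShowInventory input.
; Opening creates WBP_Inventory, adds it to the viewport, switches to Game and UI input with focus and locked mouse, and shows the cursor.
; Closing removes the widget, clears its reference and restores game-only input, so the reference's validity serves as the toggle state alongside an open flag.
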(event `self.ReceiveBeginPlay`)

(event `InputAction|ShowInventory`
  (params (Key :type "Key Structure"))
  (:`Pressed`
    (`KismetSystemLibrary.PrintString` "Hello")
    (`/Engine/EditorBlueprintResources/StandardMacros.IsValid` (`self.WBP_InventoryRef`)
      (:`Is Valid`
        (`self.Event_CloseInventory`))
      (:`Is Not Valid`
        (`self.Event_OpenInventory`)))))

(fn `Event_CloseInventory`
  (bind _wbp_inventoryref (`self.WBP_InventoryRef`))
  ;[1 1 1] Close Inventory
  (`/Engine/EditorBlueprintResources/StandardMacros.IsValid` _wbp_inventoryref
    (:`Is Valid`
      (`Widget.RemoveFromParent` _wbp_inventoryref)
      (set `self.WBP_InventoryRef` null)
      (`WidgetBlueprintLibrary.SetInputMode_GameOnly` self)
      (set `self.bShowMouseCursor` false)
      (set `self.IsInventoryOpen_0` false))))

(fn `Event_OpenInventory`
  ;[1 1 1] Open Inventory
  (`/Engine/EditorBlueprintResources/StandardMacros.IsValid` (`self.WBP_InventoryRef`)
    (:`Is Valid`
      _)
    (:`Is Not Valid`
      (bind _returnvalue (`|CreateWidget` "/Game/UserInterface/Widgets/WBP_Inventory.WBP_Inventory_C"))
      (set `self.WBP_InventoryRef` _returnvalue)))
  (`UserWidget.AddToViewport` (`self.WBP_InventoryRef`) 0)
  (`WidgetBlueprintLibrary.SetInputMode_GameAndUIEx` self (`self.WBP_InventoryRef`) "LockAlways" false)
  (set `self.bShowMouseCursor` true)
  (set `self.IsInventoryOpen_0` true))

(fn `UserConstructionScript`)