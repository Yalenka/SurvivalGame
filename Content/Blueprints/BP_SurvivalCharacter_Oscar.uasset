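; Survival character Blueprint variant "Oscar" that sets up its starting outfit when play begins.
; On authority only, BeginPlay adds one pair of cargo pants and one T-shirt to PlayerInventory.
; The same authority branch then sets the body Mesh as HelmetMesh's master pose component, so that link is not made on remote clients by this graph.
; The construction script only calls the parent.
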(event `self.ReceiveBeginPlay`
  (`/Engine/EditorBlueprintResources/ActorMacros.Switch Has Authority`
    (:`Authority`
      (`InventoryComponent.TryAddItemFromClass` (`self.PlayerInventory`) "/Game/Blueprints/Items/Gear/BP_Gear_CargoPants.BP_Gear_CargoPants_C" 1)
      (`InventoryComponent.TryAddItemFromClass` (`self.PlayerInventory`) "/Game/Blueprints/Items/Gear/BP_Gear_TShirt.BP_Gear_TShirt_C" 1)
      (`SkinnedMeshComponent.SetLeaderPoseComponent` (`self.HelmetMesh`) (`self.Mesh`) false))))

(fn `UserConstructionScript`
  (`parent.UserConstructionScript`))