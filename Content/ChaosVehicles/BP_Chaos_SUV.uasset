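; BP_Chaos_SUV is a drivable Chaos vehicle that a character can enter through its Interaction component and leave at low forward speed.
; Steering and handbrake replicate through server and multicast events, while throttle snaps to full or zero and calls multicast even on remote clients, skipping its server event.
; Entering possesses the SUV and hides the driver; exiting teleports the driver to ExitLocation and repossesses them.
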(event `Server_Throttle`
  (params (Throttle :type "Float (double-precision)"))
  ;[1 1 1] Throttle Forward/Backward
  ;;[0.4196 0 0.2824] Server and multicast :: throttle
  (`ChaosVehicleMovementComponent.SetThrottleInput` (`self.VehicleMovementComponent`) Throttle)
  (`self.Multicast_Throttle` Throttle)
  (`KismetSystemLibrary.PrintString` (`KismetStringLibrary.Conv_DoubleToString` Throttle) true true (struct :`G` 0.66 :`B` 1.0 :`A` 1.0) 0.1))

(event `InputAxis|MoveForward`
  (params (AxisValue :type "Float (single-precision)"))
  (bind _returnvalue (== AxisValue 1.0))
  (bind _returnvalue_2 (== AxisValue -1.0))
  ;[1 1 1] Throttle Forward/Backward
  (`/Engine/EditorBlueprintResources/ActorMacros.Switch Has Authority`
    (:`Authority`
      (if _returnvalue
        (`self.Multicast_Throttle` 1.0)
        (elif _returnvalue_2
          (`self.Multicast_Throttle` -1.0)
          (else
            (`self.Multicast_Throttle` 0.0)))))
    (:`Remote`
      (if _returnvalue
        (`self.Multicast_Throttle` 1.0)
        (elif _returnvalue_2
          (`self.Multicast_Throttle` -1.0)
          (else
            (`self.Multicast_Throttle` 0.0)))))))

(event `Multicast_Throttle`
  (params (Throttle :type "Float (double-precision)"))
  ;[1 1 1] Throttle Forward/Backward
  ;;[0.4196 0 0.2824] Server and multicast :: throttle
  (`ChaosVehicleMovementComponent.SetThrottleInput` (`self.VehicleMovementComponent`) Throttle)
  (`KismetSystemLibrary.PrintString` (`KismetStringLibrary.Conv_DoubleToString` Throttle) true true (struct :`G` 0.66 :`B` 1.0 :`A` 1.0) 0.1))

(event `Server_Steering`
  (params (Value :type "Float (double-precision)"))
  ;[1 1 1] Steering Left/Right
  ;;[0.4196 0 0.2824] Server and multicast :: steering
  (`ChaosVehicleMovementComponent.SetSteeringInput` (`self.VehicleMovementComponent`) Value)
  (`self.Multicast_Steering` Value))

(event `InputAxis|MoveRight`
  (params (AxisValue :type "Float (single-precision)"))
  ;[1 1 1] Steering Left/Right
  (`/Engine/EditorBlueprintResources/ActorMacros.Switch Has Authority`
    (:`Authority`
      (`self.Multicast_Steering` AxisValue))
    (:`Remote`
      (`self.Server_Steering` AxisValue))))

(event `Multicast_Steering`
  (params (Value :type "Float (double-precision)"))
  ;[1 1 1] Steering Left/Right
  ;;[0.4196 0 0.2824] Server and multicast :: steering
  (`ChaosVehicleMovementComponent.SetSteeringInput` (`self.VehicleMovementComponent`) Value))

(event `ServerHandBrake`
  (params (`New Hand Break` :type Boolean))
  ;[1 1 1] Hand Brake
  (`ChaosVehicleMovementComponent.SetHandbrakeInput` (`self.VehicleMovementComponent`) `New Hand Break`)
  (`self.MulticastHandBrake` `New Hand Break`))

(event `InputAction|Handbrake`
  (params (Key :type "Key Structure"))
  ;[1 1 1] Hand Brake
  (:`Pressed`
    (`/Engine/EditorBlueprintResources/ActorMacros.Switch Has Authority`
      (:`Authority`
        (`self.MulticastHandBrake` true))
      (:`Remote`
        (`self.ServerHandBrake` true))))
  (:`Released`
    (`/Engine/EditorBlueprintResources/ActorMacros.Switch Has Authority`
      (:`Authority`
        (`self.MulticastHandBrake` false))
      (:`Remote`
        (`self.ServerHandBrake` false)))))

(event `MulticastHandBrake`
  (params (`New Hand Break` :type Boolean))
  ;[1 1 1] Hand Brake
  (`ChaosVehicleMovementComponent.SetHandbrakeInput` (`self.VehicleMovementComponent`) `New Hand Break`))

(event `InputAxis|LookUp`
  (params (AxisValue :type "Float (single-precision)"))
  (`self.AddControllerPitchInput` (* AxisValue -1.0)))

(event `InputAxis|Turn`
  (params (AxisValue :type "Float (single-precision)"))
  (`self.AddControllerYawInput` AxisValue))

(event `self.Interaction.OnInteract`
  (params (Character :type "SurvivalCharacter Object Reference"))
  (bind _returnvalue (`self.GetController` Character))
  ;[1 1 1] Get into vehicle
  (`/Engine/EditorBlueprintResources/ActorMacros.Switch Has Authority`
    (:`Authority`
      (`KismetSystemLibrary.Delay` 0.2)
      (`Controller.Possess` _returnvalue self)
      (`self.SetOwner` _returnvalue)
      (set `self.Driver` Character)
      (`self.SetActorHiddenInGame` Character true)
      (`SceneComponent.SetHiddenInGame` (`self.Interaction`) true false))
    (:`Remote`
      (`SceneComponent.SetVisibility` (`self.Interaction`) false false))))

(event `InputAction|Interact`
  (params (Key :type "Key Structure"))
  ;[1 1 1] Exit vehicle, and limit if speed is <= 50 only exit vehicle
  (:`Pressed`
    (if (<= (`ChaosVehicleMovementComponent.GetForwardSpeed` (`self.VehicleMovementComponent`)) 50.0)
      (`self.Exit Vehicle`))))

(event `Exit Vehicle`
  ;[1 1 1] Exit vehicle, and limit if speed is <= 50 only exit vehicle
  (`self.Server Exit Vehicle`))

(event `Server Exit Vehicle`
  (bind _driver (`self.Driver`))
  ;[1 1 1] Exit vehicle, and limit if speed is <= 50 only exit vehicle
  (`self.SetActorHiddenInGame` _driver false)
  (`self.K2_SetActorLocation` _driver (`SceneComponent.K2_GetComponentLocation` (`self.ExitLocation`)) false true) ; checking teleport can fix the issue if exit location is in wall, so the player will teleport to safe location
  (`Controller.Possess` (`self.GetController`) (`self.Driver`))
  (`self.SetOwner` null)
  (set `self.Driver` null))

(fn `UserConstructionScript`)